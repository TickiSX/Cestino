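; Escapist enemy character that throws projectiles at the player (BP_Cestino) and runs away, alternating between fleeing and tired states.
; Pawn sensing triggers a throw montage and projectile spawn; when not tired it then starts fleeing and becomes tired after a delay.
; When tired, a sighting stops it, turns it red and makes it face and shoot the player before recovering.
; FleePlayer chains AI moves away from the player, re-calling itself on each success.
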(event OnSeePawn(PawnSensing)
  (params (Pawn :type Pawn%20Object%20Reference))
  (if (Variables|Default|GetIsTired?)
    (Components|Movement|StopMovementImmediately (Variables|Character|GetCharacterMovement))
    (Rendering|Material|SetMaterial (Variables|Character|GetMesh) 0 "/AnimationSharing/AnimSharingRed.AnimSharingRed")
    (bind _asbp_cestino (Utilities|Casting|CastToBP_Cestino Pawn))
    (Variables|Default|SetChar%20REF _asbp_cestino)
    (Transformation|SetActorRotation (Math|Rotator|FindLookatRotation (Transformation|GetActorLocation) (Transformation|GetActorLocation Pawn)))
    (Animation|Montage|PlayMontage (Variables|Character|GetMesh) "/Game/Characters/Escapista_Character/Animations/Lanzar_Escapista.Lanzar_Escapista"
      (:then
        (Game|SpawnActorfromClass "/Game/Levels/Level01/BP_Level/Obstacles/BP_Proyectil.BP_Proyectil_C" (Transformation|GetWorldTransform (Variables|Default|GetSpawnProyectil)) "Undefined" "SelectDefaultAtRuntime" 0 0)
        (Utilities|FlowControl|Delay 3.5)
        (Rendering|Material|SetMaterial (Variables|Character|GetMesh) 0 "/Game/Characters/Mannequins/Materials/Instances/Quinn/MI_Quinn_01.MI_Quinn_01")
        (Variables|Default|SetIsTired? false)))
    (else
      (bind _asbp_cestino_2 (Utilities|Casting|CastToBP_Cestino Pawn))
      (Variables|Default|SetChar%20REF _asbp_cestino_2)
      (Transformation|SetActorRotation (Math|Rotator|FindLookatRotation (Transformation|GetActorLocation Pawn) (Transformation|GetActorLocation Pawn)))
      (Animation|Montage|PlayMontage (Variables|Character|GetMesh) "/Game/Characters/Escapista_Character/Animations/Lanzar_Escapista.Lanzar_Escapista"
        (:then
          (Game|SpawnActorfromClass "/Game/Levels/Level01/BP_Level/Obstacles/BP_Proyectil.BP_Proyectil_C" (Transformation|GetWorldTransform (Variables|Default|GetSpawnProyectil)) "Undefined" "SelectDefaultAtRuntime" 0 0)
          (CallFunction|FleePlayer)
          (Utilities|FlowControl|Delay 7.0)
          (Variables|Default|SetIsTired? true))))))

(event Custom|FleePlayer
  (bind _returnvalue (Transformation|GetActorLocation))
  (bind _char_ref (Variables|Default|GetChar%20REF))
  (bind _returnvalue_2 (Transformation|GetActorLocation _char_ref))
  (bind _returnvalue_3 (Math|Rotator|FindLookatRotation _returnvalue _returnvalue_2))
  (bind _returnvalue_4 (Math|Vector|GetForwardVector _returnvalue_3))
  (bind _returnvalue_5 (* _returnvalue_4 -5e+02))
  (bind _returnvalue_6 (+ _returnvalue _returnvalue_5))
  (bind (_x _y) (Math|Vector|BreakVector _returnvalue_6))
  (AI|AIMoveTo self (.RandomLocation (AI|Navigation|GetRandomReachablePointinRadius (Math|Vector|MakeVector _x _y (.Z (Math|Vector|BreakVector _returnvalue))) 1e+01 0 0)) 0 5.0 false
    (:OnSuccess
      (CallFunction|FleePlayer))
    (:OnFail
      (Development|PrintString "Failed to move to position flee"))))

(fn ConstructionScript
  (|CallParentFunction))