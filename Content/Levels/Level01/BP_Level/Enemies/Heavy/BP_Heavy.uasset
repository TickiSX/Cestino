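; BP_Heavy is a heavy enemy child Blueprint that adds a punch attack.
; The Attack event plays the Punch_Heavy montage, using an IsAttaking flag to block re-entry until the montage completes.
; On the montage notify, it sphere-traces Pawn objects far forward from AttackPos and damages the hit actor, leaving debug drawing and printing on.
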(event EventAttack
  (bind _attack_pos (Variables|Default|GetAttack%20Pos))
  (bind _returnvalue (Transformation|GetWorldLocation _attack_pos))
  ;[0.15 0 0 0.5] Attack
  (if (not (Variables|Default|GetIsAttaking?))
    (Animation|Montage|PlayMontage (Variables|Character|GetMesh) "/Game/Characters/Heavy_Character/Animations/Punch_Heavy.Punch_Heavy"
      (:then
        (Variables|Default|SetIsAttaking? true))
      (:OnCompleted
        (Variables|Default|SetIsAttaking? false))
      (:OnNotifyBegin
        (bind (_outhit _returnvalue_2) (Collision|SphereTraceForObjects _returnvalue (+ _returnvalue (* (Math|Vector|GetForwardVector (Transformation|GetWorldRotation _attack_pos)) 3e+03)) 25.0 (Utilities|Array|MakeArray "ObjectTypeQuery3") false 0 "ForDuration" true "(R=1.000000,G=0.000000,B=0.000000,A=1.000000)" "(R=0.000000,G=1.000000,B=0.000000,A=1.000000)" 2.0))
        (if _returnvalue_2
          (Development|PrintString "Attack")
          (Game|Damage|ApplyDamage (.HitActor (Collision|BreakHitResult _outhit)) 1e+01 0 0))))))

(fn ConstructionScript
  (|CallParentFunction))