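; Enemy Blueprint for Level01 with an Attack event that is currently empty and an IsDead? check that always returns false.
; Disconnected attack logic sets control rotation from the look-at yaw to the player, fed into roll, and plays a headbutt montage guarded by IsAttaking.
; On the montage notify, that unused chain sphere-traces forward from AttackPos for pawns and damages the hit actor.
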(event EventAttack
  ;[0.15 0 0 0.5] Attack
)

(fn ConstructionScript
  (|CallParentFunction))

(fn IsDead?
  (return false))