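; BP_Torret is a Level01 turret obstacle that shoots at BP_Cestino when it sees it.
; PawnSensing's see-pawn event filters for that class and snaps the whole actor to face the target.
; After a short delay it spawns BP_Proyectil at the SpawnProyectil component's transform, then calls a 2D sound after a longer delay.
; Firing is paced only by sensing events and Delay nodes, with debug prints marking sighting and shot.
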(event OnSeePawn(PawnSensing)
  (params (Pawn :type Pawn%20Object%20Reference))
  (Development|PrintString "SeePlayer")
  (Utilities|Casting|CastToBP_Cestino Pawn)
  (Transformation|SetActorRotation (Math|Rotator|FindLookatRotation (Transformation|GetActorLocation) (Transformation|GetActorLocation Pawn)))
  (Utilities|FlowControl|Delay 0.75)
  (Game|SpawnActorfromClass "/Game/Levels/Level01/BP_Level/Obstacles/BP_Proyectil.BP_Proyectil_C" (Transformation|GetWorldTransform (Variables|Default|GetSpawnProyectil)) "Undefined" "SelectDefaultAtRuntime" 0 0)
  (Development|PrintString "ShootPlayer")
  (Utilities|FlowControl|Delay 2.0)
  (Audio|SpawnSound2D 0 1.0 1.0 0.0 0))

(fn ConstructionScript
  (|CallParentFunction))