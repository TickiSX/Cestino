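; BP_Proyectil is an obstacle projectile that hurts the BP_Cestino character on contact.
; On sphere overlap, it deals damage only if that character's shield is inactive, then plays a 2D sound, spawns an emitter and destroys itself.
; With the shield up it ignores the overlap; a short timer from BeginPlay also spawns an emitter and destroys it.
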(event OnComponentBeginOverlap(SphereCollision)
  (params (OverlappedComponent :type Primitive%20Component%20Object%20Reference) (OtherActor :type Actor%20Object%20Reference) (OtherComp :type Primitive%20Component%20Object%20Reference) (OtherBodyIndex :type Integer) (bFromSweep :type Boolean) (SweepResult :type Hit%20Result%20Structure%20%28by%20ref%29))
  (bind _asbp_cestino (Utilities|Casting|CastToBP_Cestino OtherActor))
  (if (not (Variables|/Game/Cestino/Blueprints/BP_Cestino.BP_Cestino_C|GetShieldActivated? _asbp_cestino))
    (Game|Damage|ApplyDamage _asbp_cestino 5.0 0 self)
    (Audio|SpawnSound2D 0 1.0 1.0 0.0 0)
    (Effects|SpawnEmitteratLocation 0 (Transformation|GetActorLocation))
    (Development|PrintString "CollisionPlayer")
    (Actor|DestroyActor)))

(event EventBeginPlay
  (Utilities|FlowControl|Delay 1.5)
  (Effects|SpawnEmitteratLocation 0 (Transformation|GetActorLocation))
  (Actor|DestroyActor))

(fn ConstructionScript)